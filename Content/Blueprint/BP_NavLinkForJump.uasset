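; Nav link proxy that makes a SoftDesignTraining main character jump to the link's destination when it reaches the smart link.
; On arrival it zeroes the character's max walk speed for a brief pause, then restores it.
; It then computes an arced velocity to the destination with SuggestProjectileVelocityCustomArc and applies it through LaunchCharacter, overriding current velocity.
; Leftover unconnected nodes, including ResumePathFollowing calls, never run.
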(event EventSmartLinkReached
  (params (Agent :type Actor%20Object%20Reference) (Destination :type Vector%20%28by%20ref%29 :default "0, 0, 0"))
  (bind _assoft_design_training_main_character (Utilities|Casting|CastToSoftDesignTrainingMainCharacter Agent))
  (Variables|Default|SetMaxSpeed (Variables|/Script/Engine.CharacterMovementComponent|GetMaxWalkSpeed (Variables|/Script/Engine.Character|GetCharacterMovement _assoft_design_training_main_character)))
  (Variables|/Script/Engine.CharacterMovementComponent|SetMaxWalkSpeed (Variables|/Script/Engine.Character|GetCharacterMovement _assoft_design_training_main_character) 0.0)
  (Utilities|FlowControl|Delay 0.3)
  (Variables|/Script/Engine.CharacterMovementComponent|SetMaxWalkSpeed (Variables|/Script/Engine.Character|GetCharacterMovement _assoft_design_training_main_character) (Variables|Default|GetMaxSpeed))
  (bind _outlaunchvelocity (Game|SuggestProjectileVelocityCustomArc (Transformation|GetActorLocation _assoft_design_training_main_character) Destination 0.0 0.5))
  (Character|LaunchCharacter _assoft_design_training_main_character _outlaunchvelocity true true))

(fn ConstructionScript)